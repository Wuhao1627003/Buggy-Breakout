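; BP_ChocolateRiver is a lethal hazard that kills the player's spud when it enters the box trigger.
; On overlap it zeroes the BP_ThirdPersonSpud's Health, destroys that actor after a short delay and shows the Death widget via ShowDeathText.
; After a further delay it clears all widgets and reloads ThirdPersonMap.
; Any other overlapping actor causes the river to destroy itself, as that DestroyActor call targets self.
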(event `self.Box.OnComponentBeginOverlap`
  (params (OverlappedComponent :type "PrimitiveComponent Object Reference") (OtherActor :type "Actor Object Reference") (OtherComp :type "PrimitiveComponent Object Reference") (OtherBodyIndex :type Integer) (bFromSweep :type Boolean) (SweepResult :type "HitResult Structure (by ref)"))
  (bind _asbp_third_person_spud (cast `/Game/BPs/BP_ThirdPersonSpud` OtherActor)
    (:`then`
      (set `/Game/BPs/BP_ThirdPersonSpud.Health` 0 _asbp_third_person_spud)
      (`KismetSystemLibrary.Delay` 1.0)
      (`self.K2_DestroyActor` OtherActor)
      (`self.ShowDeathText`)
      (`KismetSystemLibrary.Delay` 3.0)
      (`WidgetLayoutLibrary.RemoveAllWidgets`)
      (`GameplayStatics.OpenLevel` "ThirdPersonMap"))
    (:`CastFailed`
      (`self.K2_DestroyActor`))))

(fn `ShowDeathText`
  (locals (count :type Integer))
  (bind _returnvalue (`|CreateWidget` "/Game/UI/Death.Death_C"))
  (`UserWidget.AddToViewport` _returnvalue 0))

(fn `UserConstructionScript`)