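; BP_ResetArea is a trigger volume that acts as a drowning death zone, restarting the level when the player character enters it.
; On box overlap with BP_ThirdPersonSpud, it plays a drowning sound, shows the Death widget after a delay, then clears all widgets and reopens ThirdPersonMap.
; An overlap by any other actor makes the reset area destroy itself.
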(event `self.Box Collider.OnComponentBeginOverlap`
  (params (OverlappedComponent :type "PrimitiveComponent Object Reference") (OtherActor :type "Actor Object Reference") (OtherComp :type "PrimitiveComponent Object Reference") (OtherBodyIndex :type Integer) (bFromSweep :type Boolean) (SweepResult :type "HitResult Structure (by ref)"))
  (cast `/Game/BPs/BP_ThirdPersonSpud` OtherActor
    (:`then`
      (`GameplayStatics.PlaySound2D` "/Game/Sounds/drowning.drowning" 1.0 1.0 0.0 null null)
      (`KismetSystemLibrary.Delay` 1.0)
      (`self.ShowDeathText`)
      (`KismetSystemLibrary.Delay` 1.0)
      (`WidgetLayoutLibrary.RemoveAllWidgets`)
      (`GameplayStatics.OpenLevel` "ThirdPersonMap"))
    (:`CastFailed`
      (`self.K2_DestroyActor`))))

(fn `ShowDeathText`
  (bind _returnvalue (`|CreateWidget` "/Game/UI/Death.Death_C"))
  (`UserWidget.AddToViewport` _returnvalue 0))

(fn `UserConstructionScript`)