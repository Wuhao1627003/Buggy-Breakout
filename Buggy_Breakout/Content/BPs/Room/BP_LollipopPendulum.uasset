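; BP_LollipopPendulum is a lollipop pendulum that the player character can stick to.
; Any overlap with PopCollider snaps player 0's character to the StickHere socket on LollipopMain and sets OnLollipop and StartSwinging.
; Tick detaches the player, keeping world transform, once OnLollipop is false, which this graph never sets itself.
; The cached BP_ThirdPersonSpud reference feeds only disconnected logic.
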(event `self.ReceiveBeginPlay`
  (bind _asbp_third_person_spud (cast `/Game/BPs/BP_ThirdPersonSpud` (`GameplayStatics.GetPlayerCharacter` 0))))

(event `self.PopCollider.OnComponentBeginOverlap`
  (params (OverlappedComponent :type "PrimitiveComponent Object Reference") (OtherActor :type "Actor Object Reference") (OtherComp :type "PrimitiveComponent Object Reference") (OtherBodyIndex :type Integer) (bFromSweep :type Boolean) (SweepResult :type "HitResult Structure (by ref)"))
  (`self.K2_AttachToComponent` (`GameplayStatics.GetPlayerCharacter` 0) (`self.Lollipop Main`) "StickHere" "SnapToTarget" "SnapToTarget" "SnapToTarget" true)
  (set `self.OnLollipop` true)
  (set `self.StartSwinging` true))

(event `self.ReceiveTick`
  (params (DeltaSeconds :type "Float (single-precision)"))
  (if (and (not (`self.OnLollipop`)) (`self.StartSwinging`))
    (`self.K2_DetachFromActor` (`GameplayStatics.GetPlayerCharacter` 0) "KeepWorld" "KeepWorld" "KeepWorld")
    (set `self.StartSwinging` false)))

(fn `UserConstructionScript`)