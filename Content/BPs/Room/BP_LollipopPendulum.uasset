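; Lollipop pendulum that the player Spud sticks to on contact and that GrowBugs can grow.
; On BeginPlay it registers itself with the player character.
; A PopCollider hit attaches Spud to the StickHere socket on LollipopMain, or triggers Grow on that component for a GrowBug.
; Tick detaches Spud, keeping world transform, once OnLollipop is false while StartSwinging is set; nothing here clears OnLollipop.
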(event `self.ReceiveBeginPlay`
  (bind _asbp_third_person_spud (cast `/Game/BPs/BP_ThirdPersonSpud` (`GameplayStatics.GetPlayerCharacter` 0)))
  (set `/Game/BPs/BP_ThirdPersonSpud.LollipopPendulum` self _asbp_third_person_spud))

(event `self.PopCollider.OnComponentHit`
  (params (HitComponent :type "PrimitiveComponent Object Reference") (OtherActor :type "Actor Object Reference") (OtherComp :type "PrimitiveComponent Object Reference") (NormalImpulse :type "Vector Structure") (Hit :type "HitResult Structure (by ref)"))
  (bind _asbp_third_person_spud (cast `/Game/BPs/BP_ThirdPersonSpud` OtherActor)
    (:`then`
      (`KismetSystemLibrary.PrintString` "Hit Spud")
      (`self.K2_AttachToComponent` _asbp_third_person_spud (`self.Lollipop Main`) "StickHere" "SnapToTarget" "SnapToTarget" "SnapToTarget" true)
      (set `self.OnLollipop` true)
      (set `self.StartSwinging` true))
    (:`CastFailed`
      (cast `/Game/BPs/Bugs/GrowBug` OtherActor)
      (`/Game/BPs/Room/BP_Functions.Grow` (`self.Lollipop Main`)))))

(event `self.ReceiveTick`
  (params (DeltaSeconds :type "Float (single-precision)"))
  (if (and (not (`self.OnLollipop`)) (`self.StartSwinging`))
    (`self.K2_DetachFromActor` (stale `self.PopCollider.OnComponentHit` _asbp_third_person_spud) "KeepWorld" "KeepWorld" "KeepWorld")
    (set `self.StartSwinging` false)))

(fn `UserConstructionScript`)